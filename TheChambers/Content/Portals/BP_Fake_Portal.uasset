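; Fake portal variant of a parent portal Blueprint that switches off its inherited updates once its teleport trigger is touched.
; The first TeleportTrigger begin overlap sets IsItFaked through a DoOnce, with no teleport logic in this graph.
; Tick and viewport-resize events forward to the parent only while that flag is unset, and nothing here clears it.
; End overlap is empty, and construction just runs the parent script.
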(event OnComponentBeginOverlap(TeleportTrigger)
  (params (OverlappedComponent :type Primitive%20Component%20Object%20Reference) (OtherActor :type Actor%20Object%20Reference) (OtherComp :type Primitive%20Component%20Object%20Reference) (OtherBodyIndex :type Integer) (bFromSweep :type Boolean) (SweepResult :type Hit%20Result%20Structure%20%28by%20ref%29))
  (Utilities|FlowControl|DoOnce false
    (:Completed
      (Variables|Default|SetisItFaked true))))

(event OnComponentEndOverlap(TeleportTrigger)
  (params (OverlappedComponent :type Primitive%20Component%20Object%20Reference) (OtherActor :type Actor%20Object%20Reference) (OtherComp :type Primitive%20Component%20Object%20Reference) (OtherBodyIndex :type Integer)))

(event EventBeginPlay
  (|CallParentFunction) ; This node is disabled and will not be called.\nDrag off pins to build functionality.
)

(event EventOnViewportResized
  (if (not (Variables|Default|GetisItFaked))
    (|CallParentFunction)))

(event EventTick
  (params (DeltaSeconds :type Float%20%28single-precision%29))
  (if (not (Variables|Default|GetisItFaked))
    (|CallParentFunction DeltaSeconds)))

(fn ConstructionScript
  (|CallParentFunction))