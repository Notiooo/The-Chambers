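; BP_Canvas is a paintable canvas actor that records brush strokes in a runtime render target.
; On BeginPlay it creates the render target, feeds it to the canvas mesh's dynamic material and creates a dynamic brush material.
; OnPaintVisualTraceLine converts a trace hit to UV with FindCollisionUV, passes it with the brush's size, color and strength to the brush material, then draws that material into the render target.
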(event EventBeginPlay
  (bind _returnvalue (Rendering|Material|CreateDynamicMaterialInstance (Variables|Default|GetSM_Canvas) 0 "/Game/CanvasDrawingSystem/CanvasMaterialInstance.CanvasMaterialInstance" "None" :!class /Script/Engine.PrimitiveComponent))
  (bind _returnvalue_2 (Rendering|CreateRenderTarget2D (Variables|Default|GetRenderTextureSizeX) (Variables|Default|GetRenderTextureSizeY) "RTF_RGBA16f"))
  (Variables|Default|SetRenderToTexture _returnvalue_2)
  (Rendering|Material|SetTextureParameterValue _returnvalue "BrushStroke" _returnvalue_2)
  (bind _returnvalue_3 (Rendering|Material|CreateDynamicMaterialInstance "/Game/CanvasDrawingSystem/PaintBrushMaterialInstance.PaintBrushMaterialInstance" "" "None" :!class /Script/Engine.KismetMaterialLibrary))
  (Variables|Default|SetBrushMaterialInstance _returnvalue_3))

(event Collision|EventActorBeginOverlap
  (params (OtherActor :type Actor%20Object%20Reference)))

(event EventTick
  (params (DeltaSeconds :type Float%20%28single-precision%29)))

(fn ConstructionScript)

(fn OnPaintVisualTraceLine
  (params (Paint%20Brush :type BP%20Color%20Pencil%20Object%20Reference) (Hit%20Result :type Hit%20Result%20Structure))
  (bind _uv (Class|GameplayStatics|FindCollisionUV Hit%20Result))
  (bind (_x _y) (Math|Vector2D|BreakVector2D _uv))
  (Variables|Default|SetBrush Paint%20Brush)
  (Rendering|Material|SetVectorParameterValue (Variables|Default|GetBrushMaterialInstance) "HitPosition" (Utilities|Struct|MakeLinearColor _x _y 0.0 1.0) :!class /Script/Engine.MaterialInstanceDynamic)
  (Rendering|Material|SetScalarParameterValue (Variables|Default|GetBrushMaterialInstance) "BrushSize" (Variables|/Game/CanvasDrawingSystem/BP_BasePencil.BP_BasePencil_C|GetBrushSize (Variables|Default|GetBrush)) :!class /Script/Engine.MaterialInstanceDynamic)
  (Rendering|Material|SetVectorParameterValue (Variables|Default|GetBrushMaterialInstance) "BrushColor" (Variables|/Game/CanvasDrawingSystem/BP_BasePencil.BP_BasePencil_C|GetBrushColor (Variables|Default|GetBrush)) :!class /Script/Engine.MaterialInstanceDynamic)
  (Rendering|Material|SetScalarParameterValue (Variables|Default|GetBrushMaterialInstance) "BrushStrength" (Variables|/Game/CanvasDrawingSystem/BP_BasePencil.BP_BasePencil_C|GetBrushStrength (Variables|Default|GetBrush)) :!class /Script/Engine.MaterialInstanceDynamic)
  (Rendering|DrawMaterialtoRenderTarget (Variables|Default|GetRenderToTexture) (Variables|Default|GetBrushMaterialInstance)))