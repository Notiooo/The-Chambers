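; BP_Color_Pencil is a brush actor that paints on BP_Canvas actors in the canvas drawing system.
; On BeginPlay it tints its Arrow component with BrushColor.
; Every Tick it runs a short, debug-drawn complex line trace forward from the Arrow.
; When the trace hits a BP_Canvas, it passes itself and the hit result to OnPaintVisualTraceLine, leaving the painting to the canvas.
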(event EventBeginPlay
  (Components|Arrow|SetArrowColor(LinearColor) (Variables|Default|GetArrow) (Variables|Default|GetBrushColor)))

(event Collision|EventActorBeginOverlap
  (params (OtherActor :type Actor%20Object%20Reference)))

(event EventTick
  (params (DeltaSeconds :type Float%20%28single-precision%29))
  (CallFunction|DetectHitCanvasActor))

(fn ConstructionScript)

(fn DetectHitCanvasActor
  (bind _arrow (Variables|Default|GetArrow))
  (bind _returnvalue (Transformation|GetWorldLocation _arrow))
  (bind (_outhit _returnvalue_2) (Class|KismetSystemLibrary|LineTraceSinglebyProfile _returnvalue (+ _returnvalue (* (Math|Vector|GetForwardVector (Transformation|GetWorldRotation _arrow)) 15.0)) "BlockAllDynamic" true 0 "ForOneFrame" true))
  (if _returnvalue_2
    (bind _asbp_canvas (Utilities|Casting|CastToBP_Canvas (.HitActor (Collision|BreakHitResult _outhit))))
    (Default|OnPaintVisualTraceLine _asbp_canvas self _outhit)))