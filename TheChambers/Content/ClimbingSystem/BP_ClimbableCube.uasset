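; A climbable cube for VR that lets the player pull the pawn around by gripping it with motion controllers.
; Climb and LetGo track up to two gripping controllers, update the pawn's climbing-hand count and reset the pivot to the active hand.
; While climbing, Tick offsets the pawn by the active hand's drift from the pivot and pins that controller there.
; The newest grip drives movement; releasing the last stops it immediately.
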(event EventTick
  (params (DeltaSeconds :type Float%20%28single-precision%29))
  (bind _firstmotioncontroller (Variables|Default|GetFirstMotionController))
  (bind _secondmotioncontroller (Variables|Default|GetSecondMotionController))
  (bind _secondmotioncontroller_2 (Variables|Default|GetSecondMotionController))
  (bind _returnvalue (Utilities|IsValid _secondmotioncontroller_2))
  (bind _returnvalue_2 (select _returnvalue _secondmotioncontroller _firstmotioncontroller))
  (if (Utilities|IsValid (Variables|Default|GetVRPawn))
    (if (and (Variables|/Game/VRTemplate/Blueprints/VRPawn.VRPawn_C|GetisClimbing (Variables|Default|GetVRPawn)) (Utilities|IsValid (Variables|Default|GetFirstMotionController)))
      (Transformation|AddActorWorldOffset (Variables|Default|GetVRPawn) (- (Variables|Default|GetPivotPoint) (Transformation|GetWorldLocation _returnvalue_2)))
      (Transformation|SetWorldLocation _returnvalue_2 (Variables|Default|GetPivotPoint) false false))))

(event EventClimb
  (params (Motion%20Contoller :type Scene%20Component%20Object%20Reference))
  (if (Utilities|IsValid (Variables|Default|GetFirstMotionController))
    (Variables|Default|SetSecondMotionController Motion%20Contoller)
    (else
      (Variables|Default|SetFirstMotionController Motion%20Contoller)))
  (Variables|Default|SetPivotPoint (Transformation|GetWorldLocation (select (Utilities|IsValid (Variables|Default|GetSecondMotionController)) (Variables|Default|GetSecondMotionController) (Variables|Default|GetFirstMotionController))))
  (bind _asvrpawn (Utilities|Casting|CastToVRPawn (Game|Player|GetPlayerPawn 0)))
  (bind _output_get (Variables|Default|SetVRPawn _asvrpawn))
  (Math|Integer|IncrementInt (Variables|/Game/VRTemplate/Blueprints/VRPawn.VRPawn_C|GetClimbindHands _output_get)))

(event EventLetGo
  (params (Motion%20Controller :type Scene%20Component%20Object%20Reference))
  (if (Utilities|IsValid (Variables|Default|GetSecondMotionController))
    (if (== Motion%20Controller (Variables|Default|GetSecondMotionController))
      (Variables|Default|SetSecondMotionController 0)
      (Variables|Default|SetPivotPoint (Transformation|GetWorldLocation (Variables|Default|GetFirstMotionController)))
      (else
        (Variables|Default|SetFirstMotionController (Variables|Default|GetSecondMotionController))
        (Variables|Default|SetSecondMotionController 0)
        (Variables|Default|SetPivotPoint (Transformation|GetWorldLocation (Variables|Default|GetFirstMotionController)))))
    (Math|Integer|DecrementInt (Variables|/Game/VRTemplate/Blueprints/VRPawn.VRPawn_C|GetClimbindHands (Variables|Default|GetVRPawn)) :!label _label)
    (elif (== Motion%20Controller (Variables|Default|GetFirstMotionController))
      (Variables|Default|SetFirstMotionController 0)
      (Variables|Default|SetSecondMotionController 0)
      (Variables|Default|SetPivotPoint "0, 0, 0")
      (Components|Movement|StopMovementImmediately (Variables|/Script/Engine.Character|GetCharacterMovement (Variables|Default|GetVRPawn)))
      (goto _label))))

(fn ConstructionScript)

(fn AnyHold
  (return (or (Utilities|IsValid (Variables|Default|GetFirstMotionController)) (Utilities|IsValid (Variables|Default|GetSecondMotionController)))))