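; Door actor that slides open when three linked diodes are all green.
; Each tick it checks IsGreen on the three Diode references, playing a timeline if all are true and reversing it otherwise.
; The timeline's Door track drives a lerp that lowers the Cube mesh along Z, so the door closes again whenever any diode turns off.
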(event EventBeginPlay)

(event Collision|EventActorBeginOverlap
  (params (OtherActor :type Actor%20Object%20Reference)))

(event EventTick
  (params (DeltaSeconds :type Float%20%28single-precision%29))
  (if (Variables|/Game/VRTemplate/Blueprints/LaserSystem/diode.diode_C|GetisGreen (Variables|Default|Getdiode))
    (if (Variables|/Game/VRTemplate/Blueprints/LaserSystem/diode.diode_C|GetisGreen (Variables|Default|Getdiode_0))
      (if (Variables|/Game/VRTemplate/Blueprints/LaserSystem/diode.diode_C|GetisGreen (Variables|Default|Getdiode_1))
        (bind _door (Timeline|Timeline_0 Play)
          (:Update
            (Transformation|SetRelativeLocation (Variables|Default|GetCube) (Math|Vector|Lerp(Vector) "0, 0, 0" "0, 0,-101.000000" _door) false false)))
        (else
          (Timeline|Timeline_0 Reverse)))
      (else
        (Timeline|Timeline_0 Reverse)))
    (else
      (Timeline|Timeline_0 Reverse))))

(fn ConstructionScript)