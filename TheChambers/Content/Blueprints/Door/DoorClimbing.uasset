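; DoorClimbing is a door actor whose Cube slides down along its local Z when Pressed is set, then returns automatically.
; Tick polls Pressed and plays a timeline that lerps the Cube's relative location between the raised and lowered positions.
; On finish, the timeline clears Pressed and sets HasFinished, which makes a following Tick reverse it.
; Nothing in this graph sets Pressed to true.
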(event EventBeginPlay)

(event Collision|EventActorBeginOverlap
  (params (OtherActor :type Actor%20Object%20Reference)))

(event EventTick
  (params (DeltaSeconds :type Float%20%28single-precision%29))
  (if (Variables|Default|Getpressed)
    (bind _door (Timeline|Timeline_0 Play)
      (:Update
        (Transformation|SetRelativeLocation (Variables|Default|GetCube) (Math|Vector|Lerp(Vector) "0, 0, 0" "0, 0,-101.000000" _door) false false))
      (:Finished
        (Variables|Default|SethasFinished true)
        (Variables|Default|Setpressed false)))
    (elif (Variables|Default|GethasFinished)
      (Variables|Default|SethasFinished false)
      (Timeline|Timeline_0 Reverse))))

(fn ConstructionScript)