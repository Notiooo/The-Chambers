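; Door actor that slides its Cube component down to open and back up to close.
; Open and Close functions only set request flags, which Tick polls to start a timed, relative MoveComponentTo.
; State flags block repeat moves while the door is already moving to or resting in the requested state.
; Tick also clamps the cube's relative Z between two variable limits to contain the relative offsets.
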(event EventBeginPlay)

(event Collision|EventActorBeginOverlap
  (params (OtherActor :type Actor%20Object%20Reference)))

(event EventTick
  (params (DeltaSeconds :type Float%20%28single-precision%29))
  (bind _newvar_0 (Variables|Default|GetNewVar_0))
  (bind _newvar_1 (Variables|Default|GetNewVar_1))
  (bind _cube (Variables|Default|GetCube))
  (bind _cube_2 (Variables|Default|GetCube))
  (bind _relativelocation (Variables|/Script/Engine.SceneComponent|GetRelativeLocation _cube))
  (bind _relativelocation_2 (Variables|/Script/Engine.SceneComponent|GetRelativeLocation _cube_2))
  (if (> (.z _relativelocation_2) _newvar_1)
    (Transformation|SetRelativeLocation _cube_2 (Math|Vector|MakeVector (.x _relativelocation_2) (.y _relativelocation_2) _newvar_1) false true)
    (elif (< (.z _relativelocation_2) _newvar_0)
      (Transformation|SetRelativeLocation _cube_2 (Math|Vector|MakeVector (.x _relativelocation_2) (.y _relativelocation_2) _newvar_0) false true)))
  (if (Variables|Default|GetshouldOpen)
    (if (not (Variables|Default|GetisOpen))
      (if (not (Variables|Default|GetisOpening))
        (Variables|Default|SetisClose false)
        (Variables|Default|SetisOpening true)
        (Components|MoveComponentTo _cube (- _relativelocation "0, 0,300.000000") "0, 0, 0" false false 0.5 false)
        (Variables|Default|SetisOpen true)
        (Variables|Default|SetisOpening false)
        (Variables|Default|SetisClose false)))
    (elif (Variables|Default|GetshouldClose)
      (if (not (Variables|Default|GetisClose))
        (if (not (Variables|Default|GetisClosing))
          (Variables|Default|SetisOpen false)
          (Variables|Default|SetisClosing true)
          (Components|MoveComponentTo _cube (- _relativelocation "0, 0,-300.000000") "0, 0, 0" false false 0.5 false)
          (Variables|Default|SetisClose true)
          (Variables|Default|SetisClosing false)
          (Variables|Default|SetisOpen false))))))

(fn ConstructionScript)

(fn Open
  (Variables|Default|SetshouldOpen true)
  (Variables|Default|SetshouldClose false))

(fn Close
  (Variables|Default|SetshouldClose true)
  (Variables|Default|SetshouldOpen false))