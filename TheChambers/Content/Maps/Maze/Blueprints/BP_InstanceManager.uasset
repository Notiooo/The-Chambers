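; BP_InstanceManager is an actor in the Maze map's Blueprints that manages instanced static meshes, grouping placed copies by mesh asset.
; A map links each mesh to its own Hierarchical Instanced Static Mesh component, which is created the first time that mesh is added.
; Its functions add world-space instances and return their index, remove one by mesh and index, or clear instances for one or all meshes.
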(event EventBeginPlay)

(event Collision|EventActorBeginOverlap
  (params (OtherActor :type Actor%20Object%20Reference)))

(event EventTick
  (params (DeltaSeconds :type Float%20%28single-precision%29)))

(fn ConstructionScript)

(fn AddNewMeshInstance
  (params (Mesh :type Static%20Mesh%20Object%20Reference) (Transform :type Transform))
  (bind _instancecomponent_list (Variables|Default|GetInstanceComponent_List))
  (bind (_value _returnvalue) (Utilities|Map|Find _instancecomponent_list Mesh))
  (if _returnvalue
    (bind _returnvalue_2 (Class|InstancedStaticMeshComponent|AddInstanceWorldSpace _value Transform))
    (return true _returnvalue_2)
    (else
      (bind _returnvalue_3 (AddComponent|AddHierarchicalInstancedStaticMeshComponent false))
      (Utilities|Map|Add (Variables|Default|GetInstanceComponent_List) Mesh _returnvalue_3)
      (Components|StaticMesh|SetStaticMesh _returnvalue_3 Mesh)
      (bind _returnvalue_4 (Class|InstancedStaticMeshComponent|AddInstanceWorldSpace _returnvalue_3 Transform))
      (return true _returnvalue_4))))

(fn RemoveAllInstances
  (bind _keys (Utilities|Map|Keys (Variables|Default|GetInstanceComponent_List)))
  (for _array_element _keys
    (Components|InstancedStaticMesh|ClearInstances (.Value (Utilities|Map|Find (Variables|Default|GetInstanceComponent_List) _array_element))))
  (return true))

(fn RemoveAllMeshInstances
  (params (Mesh :type Static%20Mesh%20Object%20Reference))
  (bind _instancecomponent_list (Variables|Default|GetInstanceComponent_List))
  (bind (_value _returnvalue) (Utilities|Map|Find _instancecomponent_list Mesh))
  (if _returnvalue
    (Components|InstancedStaticMesh|ClearInstances _value)
    (return true)
    (else
      (return false))))

(fn RemoveMeshInstance
  (params (Mesh :type Static%20Mesh%20Object%20Reference) (index :type Integer))
  (bind _instancecomponent_list (Variables|Default|GetInstanceComponent_List))
  (bind (_value _returnvalue) (Utilities|Map|Find _instancecomponent_list Mesh))
  (if _returnvalue
    (bind _returnvalue_2 (Class|InstancedStaticMeshComponent|RemoveInstance _value index))
    (return _returnvalue_2)
    (else
      (return false))))