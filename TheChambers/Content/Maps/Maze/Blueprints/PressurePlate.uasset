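; Pressure plate for the Maze map that reacts when a VRPawn steps into or out of its box trigger.
; On overlap begin it sets IsPressed, briefly animates the button slightly downward and calls Reset.
; On overlap end it clears IsPressed and raises the button by the same offset.
; Both moves are relative to the button's current position rather than a stored rest position.
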(event OnComponentBeginOverlap(Box)
  (params (OverlappedComponent :type Primitive%20Component%20Object%20Reference) (OtherActor :type Actor%20Object%20Reference) (OtherComp :type Primitive%20Component%20Object%20Reference) (OtherBodyIndex :type Integer) (bFromSweep :type Boolean) (SweepResult :type Hit%20Result%20Structure%20%28by%20ref%29))
  (bind _button (Variables|Default|GetButton))
  (bind _returnvalue (Transformation|GetRelativeTransform _button))
  (Utilities|Casting|CastToVRPawn OtherActor)
  (Variables|Default|SetisPressed true)
  (Components|MoveComponentTo _button (- (.location _returnvalue) "0, 0,0.200000") (.rotation _returnvalue) false false 0.1 false)
  (Default|CallReset))

(event OnComponentEndOverlap(Box)
  (params (OverlappedComponent :type Primitive%20Component%20Object%20Reference) (OtherActor :type Actor%20Object%20Reference) (OtherComp :type Primitive%20Component%20Object%20Reference) (OtherBodyIndex :type Integer))
  (bind _button (Variables|Default|GetButton))
  (bind _returnvalue (Transformation|GetRelativeTransform _button))
  (Utilities|Casting|CastToVRPawn OtherActor)
  (Variables|Default|SetisPressed false)
  (Components|MoveComponentTo _button (- (.location _returnvalue) "0, 0,-0.200000") (.rotation _returnvalue) false false 0.1 false))

(event Collision|EventActorBeginOverlap
  (params (OtherActor :type Actor%20Object%20Reference)))

(event EventTick
  (params (DeltaSeconds :type Float%20%28single-precision%29)))

(fn ConstructionScript)