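; RiddleManager is an actor in the Doors map that starts the correct riddle when a VRPawn enters its trigger box.
; The first overlap plays a 2D introduction sound, waits for its duration, then sets ShouldPlay on the selected riddle.
; CorrectRiddleID selects among three stored riddle references, which SetRiddles assigns, with the third as fallback.
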(event OnComponentBeginOverlap(Box)
  (params (OverlappedComponent :type Primitive%20Component%20Object%20Reference) (OtherActor :type Actor%20Object%20Reference) (OtherComp :type Primitive%20Component%20Object%20Reference) (OtherBodyIndex :type Integer) (bFromSweep :type Boolean) (SweepResult :type Hit%20Result%20Structure%20%28by%20ref%29))
  (bind _introductionsound (Variables|Default|GetIntroductionSound))
  (Utilities|Casting|CastToVRPawn OtherActor)
  (bind _correctriddle (CallFunction|GetCorrectRiddle))
  (Utilities|FlowControl|DoOnce false
    (:Completed
      (Audio|PlaySound2D _introductionsound 1.0 1.0 0.0 0 0)
      (Utilities|FlowControl|Delay (Variables|/Script/Engine.SoundBase|GetDuration _introductionsound))
      (Variables|/Game/Maps/3_Doors/Blueprints/Riddle.Riddle_C|SetshouldPlay _correctriddle true))))

(event EventBeginPlay)

(event Collision|EventActorBeginOverlap
  (params (OtherActor :type Actor%20Object%20Reference)))

(event EventTick
  (params (DeltaSeconds :type Float%20%28single-precision%29)))

(fn ConstructionScript)

(fn GetCorrectRiddle
  (bind _correctriddleid (Variables|Default|GetCorrectRiddleID))
  (if (== _correctriddleid 1)
    (return (Variables|Default|GetRiddleOne))
    (elif (== _correctriddleid 2)
      (return (Variables|Default|GetRiddleTwo))
      (else
        (return (Variables|Default|GetRiddleThree))))))

(fn SetRiddles
  (params (NewParam :type Riddle%20Object%20Reference%20%28by%20ref%29) (NewParam1 :type Riddle%20Object%20Reference%20%28by%20ref%29) (NewParam2 :type Riddle%20Object%20Reference%20%28by%20ref%29))
  (Variables|Default|SetRiddleOne NewParam)
  (Variables|Default|SetRiddleTwo NewParam1)
  (Variables|Default|SetRiddleThree NewParam2))